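; Player controller that toggles between the Candleboy character and a photo-mode camera pawn.
; BeginPlay caches the controlled pawn and spawns a hidden BP_Camera at its transform.
; A FlipFlop on the IA_ToggleCamera input alternates possession and visibility between the two.
; Entering photo mode passes Candleboy's location to the camera, while exiting moves Candleboy to the location the camera's Exit returns.
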(event Input|EnhancedActionEvents|EnhancedInputActionIA_ToggleCamera
  (params (ActionValue :type Boolean) (ElapsedSeconds :type Float%20%28double-precision%29) (TriggeredSeconds :type Float%20%28double-precision%29) (InputAction :type Input%20Action%20Object%20Reference :default "/Game/Assets/CandleBoy/Input/Actions/IA_ToggleCamera.IA_ToggleCamera"))
  (bind _cameraactor (Variables|Default|GetCameraActor))
  (bind _candleboy_ref (Variables|Default|GetCandleboy%20Ref))
  (bind _candleboy_ref_2 (Variables|Default|GetCandleboy%20Ref))
  ;[1 1 1] Every time we switch the camera, we are going through a flipflop. This will switch between the A & B on every time it is entered.
  ;
  ; We can use which one it is to switch between the Original Pawn (Candleboy) and the Camera actor we created on begin play. We can also use it to hide and unhide each actor individually using the boolean.
  (:Completed
    (bind _isa (Utilities|FlowControl|FlipFlop)
      (:A
        _)
      (:B
        _))
    (Rendering|SetActorHiddenInGame _candleboy_ref true)
    (Pawn|Possess (select _isa _cameraactor _candleboy_ref))
    (Rendering|SetActorHiddenInGame (select _isa _cameraactor _candleboy_ref) false)
    (if _isa
      (Default|EnterPhotoMode _cameraactor (Transformation|GetActorLocation _candleboy_ref_2))
      (else
        (bind _location (Default|Exit _cameraactor))
        (Transformation|SetActorLocation _candleboy_ref_2 _location false false)))))

(event EventBeginPlay
  (bind _returnvalue (Pawn|GetControlledPawn))
  (bind _self self)
  ;[1 1 1] Create a reference to CandleBoy on begin play and then create a new instance of the Camera Actor Class which we immediately hide.
  (Variables|Default|SetCandleboy%20Ref _returnvalue)
  (bind _returnvalue_2 (Game|SpawnActorfromClass "/Game/Assets/Camera/BP_Camera.BP_Camera_C" (Transformation|GetActorTransform _returnvalue) "Undefined" _self _self))
  (bind _output_get (Variables|Default|SetCameraActor _returnvalue_2))
  (Rendering|SetActorHiddenInGame _output_get true))

(fn ConstructionScript)